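; BP_Blackhole is the Blackhole action, gated by and paid for with the instigator's Rage attribute.
; CanStart extends the parent check by requiring Rage to cover RageCost, printing a message when it falls short.
; StartAction runs the parent behavior, then deducts RageCost through the attribute component's ApplyRageChange.
; The graphs here add only the resource cost, with any black hole effect left outside them.
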(event EventStartAction
  (params (InstigatorActor :type Actor%20Object%20Reference))
  (|CallParentFunction InstigatorActor)
  (bind _returnvalue (Class|SAttributeComponent|GetAttributes InstigatorActor))
  (Class|SAttributeComponent|ApplyRageChange _returnvalue InstigatorActor (* (Variables|Default|GetRageCost) -1.0)))

(fn CanStart
  (params (InstigatorActor :type Actor%20Object%20Reference))
  (bind _returnvalue (|CallParentFunction InstigatorActor))
  (if _returnvalue
    (bind _returnvalue_2 (Class|SAttributeComponent|GetAttributes InstigatorActor))
    (if (>= (Variables|/Script/RogueLike.SAttributeComponent|GetRage _returnvalue_2) (Variables|Default|GetRageCost))
      (return true)
      (else
        (Development|PrintString "Not enough rage")
        (return false)))
    (else
      (return false))))