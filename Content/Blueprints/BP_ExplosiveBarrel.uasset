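; Explosive barrel actor that blows up when its static mesh registers a hit, with the explosion routed through a network authority check.
; On authority it calls the multicast explosion and sets a short lifespan for cleanup, while the remote branch calls the custom event that re-enters the same check.
; The explosion event prints a debug string, fires a RadialForce impulse, then disables collision and hides the actor.
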(event OnComponentHit(StaticMeshComponent)
  (params (HitComponent :type Primitive%20Component%20Object%20Reference) (OtherActor :type Actor%20Object%20Reference) (OtherComp :type Primitive%20Component%20Object%20Reference) (NormalImpulse :type Vector :default "0, 0, 0") (Hit :type Hit%20Result%20Structure%20%28by%20ref%29))
  (Networking|SwitchHasAuthority
    (:Authority
      (CallFunction|MulticastExplosion)
      (Actor|SetLifeSpan 2.0))
    (:Remote
      (CallFunction|CustomEvent))))

(event Custom|Multicast_Explosion
  (Development|PrintString "Explode!" true false)
  (Class|RadialForceComponent|FireImpulse (Variables|Default|GetRadialForce))
  (Collision|SetActorEnableCollision false)
  (Rendering|SetActorHiddenInGame true))

(event Custom|CustomEvent
  (Networking|SwitchHasAuthority
    (:Authority
      (CallFunction|MulticastExplosion)
      (Actor|SetLifeSpan 2.0))
    (:Remote
      (CallFunction|CustomEvent))))

(fn ConstructionScript)