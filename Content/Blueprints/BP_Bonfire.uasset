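; BP_Bonfire is an interactable bonfire that acts as a save point.
; Interact marks the fire active, writes the save game through SGameModeBase and calls BeginFlames.
; OnActorLoaded also calls BeginFlames, which activates the particle system only when IsFireActive is set, so a lit fire shows its flames again after loading.
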(event EventInteract
  (params (InstigatorPawn :type Pawn%20Object%20Reference))
  (Variables|Default|SetbIsFireActive true)
  (Class|SGameModeBase|WriteSaveGame (.AsSGame%20Mode%20Base (Utilities|Casting|CastToSGameModeBase (Game|GetGameMode))))
  (CallFunction|BeginFlames))

(event EventOnActorLoaded
  (CallFunction|BeginFlames))

(fn ConstructionScript)

(fn BeginFlames
  (if (Variables|Default|GetbIsFireActive)
    (Components|Activation|Activate (Variables|Default|GetParticleSystem) false)))